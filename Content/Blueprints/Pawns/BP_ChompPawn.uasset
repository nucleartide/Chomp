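; BP_ChompPawn is a pawn whose top and bottom halves rotate in opposite directions to animate a chomping mouth.
; The ChompAnimation timeline starts on BeginPlay at a configurable rate, and its value scales DegreesToRotate to set each half's pitch.
; Tick polls ChompPlayerController's IsMoving, playing the timeline while moving and stopping it in place otherwise.
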(event `self.ReceiveBeginPlay`
  (`TimelineComponent.SetPlayRate` (`self.ChompAnimation`) (`self.AnimationRate`))
  (bind (_direction _rotationvalue) (`Timeline|ChompAnimation`)
    (:`Update`
      (bind _returnvalue (* _rotationvalue (`self.DegreesToRotate`)))
      (`SceneComponent.K2_SetRelativeRotation` (`self.BottomHalf`) (`KismetMathLibrary.MakeRotator` 0.0 (- 360.0 _returnvalue)) false false)
      (`SceneComponent.K2_SetRelativeRotation` (`self.TopHalf`) (`KismetMathLibrary.MakeRotator` 0.0 (+ 180.0 _returnvalue)) false false))))

(event `self.ReceiveTick`
  (params (DeltaSeconds :type "Float (single-precision)"))
  (bind _returnvalue (`self.GetController`))
  (`/Engine/EditorBlueprintResources/StandardMacros.IsValid` _returnvalue
    (:`Is Valid`
      (bind _aschomp_player_controller (cast `ChompPlayerController` _returnvalue)
        (:`then`
          (if (`ChompPlayerController.IsMoving` _aschomp_player_controller)
            (if (not (`TimelineComponent.IsPlaying` (`self.ChompAnimation`)))
              (`TimelineComponent.Play` (`self.ChompAnimation`)))
            (else
              (`TimelineComponent.Stop` (`self.ChompAnimation`)))))
        (:`CastFailed`
          (`KismetSystemLibrary.PrintString` "Failed to cast to ChompPlayerController. See BP_ChompPawn." true true (struct :`R` 1.0 :`B` 0.038955 :`A` 1.0) 5.0))))))

(fn `UserConstructionScript`)