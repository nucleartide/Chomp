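; Camera actor that becomes the first player's view and sets its own aspect ratio when play begins.
; On BeginPlay it makes itself player controller 0's view target, then configures its camera component.
; The aspect ratio is a fixed 16:10 on Mac and is derived from the desktop resolution on other platforms.
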(event `self.ReceiveBeginPlay`
  (`PlayerController.SetViewTargetWithBlend` (`GameplayStatics.GetPlayerController` 0) self 0.0 "VTBlend_Linear" 0.0 false)
  (if (`KismetStringLibrary.EqualEqual_StrStr` (`GameplayStatics.GetPlatformName`) "Mac")
    (`CameraComponent.SetAspectRatio` (`self.CameraComponent`) 1.6)
    (else
      (bind _returnvalue (`GameUserSettings.GetGameUserSettings`))
      (bind (_x _y) (break `IntPoint` (`GameUserSettings.GetDesktopResolution` _returnvalue)))
      (`CameraComponent.SetAspectRatio` (`self.CameraComponent`) (`KismetMathLibrary.SafeDivide` (`KismetMathLibrary.Conv_IntToDouble` _x) (`KismetMathLibrary.Conv_IntToDouble` _y))))))

(fn `UserConstructionScript`)